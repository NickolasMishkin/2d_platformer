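; Flying platform actor meant to shuttle between two endpoints, taken from the world positions of two arrow components at BeginPlay.
; Tick counts down a wait timer, then on arrival flips the destination and restarts the wait, snapping to the nearer endpoint if off both.
; Arrival checks use a tolerance scaled by speed and frame time.
; No incremental movement is wired, and leftover replication and position-reset fragments never run.
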(event EventBeginPlay
  (Variables|Default|Setpos1 (Transformation|GetWorldLocation (Variables|Default|GetArrow_1)))
  (Variables|Default|Setpos2 (Transformation|GetWorldLocation (Variables|Default|GetArrow_2)))
  (bind _output_get (Variables|Default|Setcpos (Variables|Default|Getpos1)))
  (Variables|Default|Setdesloc _output_get))

(event EventTick
  (params (DeltaSeconds :type Float%20%28single-precision%29))
  (bind _pos1 (Variables|Default|Getpos1))
  (bind _pos2 (Variables|Default|Getpos2))
  (Variables|Default|Setdt DeltaSeconds)
  (if (<= (Variables|Default|Getwait) 0.0)
    (Utilities|FlowControl|Sequence
      (:then_1
        (if (Math|Vector|Equal(Vector) (Variables|Default|Getdesloc) (Variables|Default|Getcpos) (* (Variables|Default|Getspd) (Variables|Default|Getdt) 0.51))
          (if (Math|Vector|Equal(Vector) (Variables|Default|Getdesloc) (Variables|Default|Getpos1) (* (Variables|Default|Getspd) (Variables|Default|Getdt) 0.51))
            (Variables|Default|Setdesloc (Variables|Default|Getpos2))
            (Variables|Default|Setsloc (Variables|Default|Getpos1))
            (Variables|Default|Setwait (Variables|Default|Getwaittime))
            (elif (Math|Vector|Equal(Vector) (Variables|Default|Getdesloc) (Variables|Default|Getpos2) (* (Variables|Default|Getspd) (Variables|Default|Getdt) 0.51))
              (Variables|Default|Setdesloc (Variables|Default|Getpos1))
              (Variables|Default|Setsloc (Variables|Default|Getpos2))
              (Variables|Default|Setwait (Variables|Default|Getwaittime))
              (else
                (if (> (Math|Vector|VectorLength (- (Variables|Default|Getpos1) (Variables|Default|Getdesloc))) (Math|Vector|VectorLength (- (Variables|Default|Getpos2) (Variables|Default|Getdesloc))))
                  (Variables|Default|Setepos _pos2)
                  (Variables|Default|Setdesloc _pos1)
                  (else
                    (Variables|Default|Setepos _pos1)
                    (Variables|Default|Setdesloc _pos2)))
                (Transformation|SetActorLocation (Variables|Default|Getepos) false false)
                (Variables|Default|Setcpos (Variables|Default|Getepos))))))))
    (else
      (Variables|Default|Setwait (- (Variables|Default|Getwait) (Variables|Default|Getdt))))))

(fn ConstructionScript)
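; PlayerBullet is the player's projectile in a 2D side-scroller, dealing damage to what it touches.
; On BeginPlay it copies DirX from the 2DSideScrollerCharacter and snaps to the player pawn's location.
; Tick moves it along X at Speed in that fixed direction, setting location directly without sweep.
; Any actor overlap applies Dmg and destroys the bullet, with no target filter or lifetime limit.
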(event EventBeginPlay
  (bind _as2dside_scroller_character (Utilities|Casting|CastTo2DSideScrollerCharacter (Game|Player|GetPlayerPawn 0)))
  (bind _output_get (Variables|Default|Setplayer _as2dside_scroller_character))
  (Variables|Default|Setkx (Variables|/Game/Blueprints/2DSideScrollerCharacter.2DSideScrollerCharacter_C|GetdirX _output_get))
  (Transformation|SetActorLocation (Transformation|GetActorLocation (Game|Player|GetPlayerPawn 0)) false false))

(event Collision|EventActorBeginOverlap
  (params (OtherActor :type Actor%20Object%20Reference))
  (Game|Damage|ApplyDamage OtherActor (Variables|Default|Getdmg) 0 0)
  (Actor|DestroyActor))

(event EventTick
  (params (DeltaSeconds :type Float%20%28single-precision%29))
  (bind _returnvalue (Transformation|GetActorLocation))
  (bind (_x _y _z) (Math|Vector|BreakVector _returnvalue))
  (Transformation|SetActorLocation (Math|Vector|MakeVector (+ _x (* (Variables|Default|Getspeed) DeltaSeconds (Math|Conversions|ToFloat(Integer) (Variables|Default|Getkx)))) _y _z) false false))

(fn ConstructionScript)
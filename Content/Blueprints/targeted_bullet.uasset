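; Enemy projectile Blueprint that fires toward the position the player pawn occupies when the bullet spawns.
; BeginPlay caches that target and the origin, then Tick feeds both into a Movement helper with speed and delta time to reposition the bullet without sweeping.
; Hits use a distance check against the player's current location instead of collision, applying damage and destroying the bullet, which also destroys itself when its lifetime expires.
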(event EventBeginPlay
  (Variables|Default|Settarget (Transformation|GetActorLocation (Game|Player|GetPlayerPawn 0)))
  (bind _output_get (Variables|Default|Setorigin (Transformation|GetActorLocation)))
  (Variables|Default|Setcloc _output_get))

(event Collision|EventActorBeginOverlap
  (params (OtherActor :type Actor%20Object%20Reference)))

(event EventTick
  (params (DeltaSeconds :type Float%20%28single-precision%29))
  (bind _output_get (Variables|Default|Setdt DeltaSeconds))
  (Variables|Default|Setlife (- (Variables|Default|Getlife) _output_get))
  (if (> (Variables|Default|Getlife) 0.0)
    (bind _n_loc (CallFunction|Movement (Variables|Default|Gettarget) (Variables|Default|Getorigin) (Variables|Default|Getcloc) (Variables|Default|Getspd) (Variables|Default|Getdt)))
    (bind _output_get_2 (Variables|Default|Setcloc _n_loc))
    (Transformation|SetActorLocation _output_get_2 false false)
    (bind _d (CallFunction|Getdist (Transformation|GetActorLocation (Game|Player|GetPlayerPawn 0)) (Variables|Default|Getcloc)))
    (if (< _d 15.0)
      (Game|Damage|ApplyDamage (Game|Player|GetPlayerPawn 0) (Variables|Default|Getdmg) 0 0)
      (Actor|DestroyActor))
    (else
      (Actor|DestroyActor))))

(fn ConstructionScript)